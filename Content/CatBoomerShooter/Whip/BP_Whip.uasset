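; Player whip melee weapon that attaches to the character's grip point and stays hidden except while attacking.
; PrimaryAttack runs a three-step combo, using timelines to rotate the whip while its capsule gathers overlapping enemies.
; When the swing finishes, those enemies take damage and knockback, much stronger on the third slash, before a reverse timeline retracts the whip.
; Hits advance the combo, which resets after the third or when a timer expires.
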(event Custom|ResetCombo
  (Variables|Default|SetAttackCombo 1))

(event Custom|PrimaryAttack
  (if (not (Variables|Default|GetAttacking?))
    (Variables|Default|SetAttacking? true)
    (Rendering|SetActorHiddenInGame self false)
    (switch int (Variables|Default|GetAttackCombo)
      (:1
        (bind _y_rotation (Timeline|Timeline_MainAttack PlayFromStart)
          (:Update
            (Transformation|SetActorRelativeRotation (Math|Rotator|MakeRotator 0.0 _y_rotation 0.0))
            (for _array_element (Collision|GetOverlappingActors (Variables|Default|GetCapsule) "/Game/CatBoomerShooter/Enemy/BP_Enemy.BP_Enemy_C" :!class /Script/Engine.PrimitiveComponent) :!label _label
              (Utilities|Array|AddUnique (Variables|Default|GetEnemiesHit) _array_element)))
          (:Finished
            (for _array_element_2 (Variables|Default|GetEnemiesHit) :!label _label_2
              (bind _asbp_enemy (Utilities|Casting|CastToBP_Enemy _array_element_2))
              (Variables|/Game/CatBoomerShooter/Enemy/BP_Enemy.BP_Enemy_C|SetHealth _asbp_enemy (- (Variables|/Game/CatBoomerShooter/Enemy/BP_Enemy.BP_Enemy_C|GetHealth _asbp_enemy) (Variables|Default|GetDamage)))
              (switch int (Variables|Default|GetAttackCombo)
                (:1
                  (Character|LaunchCharacter _asbp_enemy (* (Transformation|GetActorForwardVector (Game|GetPlayerCharacter 0)) (Variables|Default|GetKnockbackPower)) false false :!label _label_3))
                (:2
                  (goto _label_3))
                (:3
                  (Character|LaunchCharacter _asbp_enemy (* (Transformation|GetActorForwardVector (Game|GetPlayerCharacter 0)) (* (Variables|Default|GetKnockbackPower) 5)) false false))))
            (switch int (Variables|Default|GetAttackCombo)
              (:1
                (bind _y_rotation_2 (Timeline|ReverseTimeline_MainAttack ReverseFromEnd)
                  (:Update
                    (Transformation|SetActorRelativeRotation (Math|Rotator|MakeRotator 0.0 _y_rotation_2 0.0)))
                  (:Finished
                    (Utilities|FlowControl|Sequence :!label _label_4
                      (:then_0
                        (if (Utilities|Array|IsNotEmpty (Variables|Default|GetEnemiesHit))
                          (bind _result (Math|Integer|IncrementInt (Variables|Default|GetAttackCombo))
                            (:%20%20
                              (if (> _result 3)
                                (Utilities|Time|ClearandInvalidateTimerbyHandle (Variables|Default|GetCountdownTimer))
                                (CallFunction|ResetCombo)
                                (else
                                  (if (Utilities|Time|IsValidTimerHandle (Variables|Default|GetCountdownTimer))
                                    (Utilities|Time|ClearandInvalidateTimerbyHandle (Variables|Default|GetCountdownTimer)))
                                  (bind _returnvalue (Utilities|Time|SetTimerbyEvent (delegate Custom|ResetCombo) 2.0))
                                  (Variables|Default|SetCountdownTimer _returnvalue)))))))
                      (:then_1
                        (Variables|Default|SetAttacking? false)
                        (Utilities|Array|Clear (Variables|Default|GetEnemiesHit))
                        (Rendering|SetActorHiddenInGame self true))))))
              (:2
                (Timeline|ReverseTimeline_MainAttack ReverseFromEnd))
              (:3
                (bind (_direction _x_rotation _y_rotation_3) (Timeline|ReverseTimeline_SlashAttack ReverseFromEnd)
                  (:Update
                    (Transformation|SetActorRelativeRotation (Math|Rotator|MakeRotator _x_rotation _y_rotation_3 0.0)))
                  (:Finished
                    (goto _label_4))))))))
      (:2
        (Timeline|Timeline_MainAttack PlayFromStart))
      (:3
        (bind (_direction_2 _x_rotation_2 _y_rotation_4) (Timeline|Timeline_SlashAttack PlayFromStart)
          (:Update
            (Transformation|SetActorRelativeRotation (Math|Rotator|MakeRotator _x_rotation_2 _y_rotation_4 0.0))
            (goto _label))
          (:Finished
            (goto _label_2)))))))

(event EventBeginPlay
  (bind _returnvalue (Class|BasePlayerInterface|GetPlayerWhipLocation(Message) (Game|GetPlayerCharacter 0)))
  (Utilities|IsValid _returnvalue
    (:Is%20Valid
      (Transformation|AttachComponentToComponent _returnvalue "GripPoint" "SnapToTarget" "SnapToTarget" "SnapToTarget" true)
      (Rendering|SetActorHiddenInGame self true))))

(fn ConstructionScript)