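; BP_TestTrain is a test train that moves a static mesh along a spline in a continuous loop.
; Each Tick advances a distance by Speed and DeltaSeconds, then sets the mesh's world transform from the spline at that distance.
; Once the distance exceeds the spline length, the mesh teleports to the first spline point and the distance resets to zero.
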(event EventTick
  (params (DeltaSeconds :type Float%20%28single-precision%29))
  (bind _spline (Variables|Default|GetSpline))
  (Variables|Default|SetDistance (+ (* DeltaSeconds (Variables|Default|GetSpeed)) (Variables|Default|GetDistance)))
  (Transformation|SetWorldTransform (Variables|Default|GetStaticMesh) (Spline|GetTransformatDistanceAlongSpline _spline (Variables|Default|GetDistance) "World" false) false false)
  (if (> (Variables|Default|GetDistance) (Spline|GetSplineLength _spline))
    ;[1 1 1] Teleport function
    (Transformation|SetRelativeTransform (Variables|Default|GetStaticMesh) (Spline|GetTransformatSplinePoint (Variables|Default|GetSpline) 0 "Local" false) false true)
    (Variables|Default|SetDistance 0.0)))

(fn ConstructionScript)