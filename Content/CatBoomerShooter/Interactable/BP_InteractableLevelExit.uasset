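; BP_InteractableLevelExit is an interactable exit that takes the player to another level.
; When a BasePlayerCharacter interacts with it, OnInteract fires OnInteractSave and reports success.
; That event saves actors asynchronously and opens the referenced level only once the save completes.
; The construction script shows LevelName on the exit's text render component.
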(event Custom|OnInteractSave
  (|AsyncSaveActors 1
    (:OnCompleted
      (Game|OpenLevel(byObjectReference) (Variables|Default|GetLevelRef)))))

(fn ConstructionScript
  (Rendering|Components|TextRender|SetText (Variables|Default|GetTextRender) (Variables|Default|GetLevelName)))

(fn OnInteract
  (params (OwningActor :type Actor%20Object%20Reference))
  (Utilities|Casting|CastToBasePlayerCharacter OwningActor)
  (CallFunction|OnInteractSave)
  (return true))