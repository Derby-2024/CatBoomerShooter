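; Player grapple hook component that pulls the owning character toward BP_GrappleHookTarget actors.
; A tick-driven state machine highlights the visible in-range target closest to camera aim while inactive.
; Grapple input spawns a hook and cable toward an on-screen target; hook proximity triggers a hop, then accelerating velocity pulls the character in once rising stops.
; Arrival launches a final hop; arrival, jump or re-pressing grapple cleans up and updates arms animation.
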(event Input|EnhancedActionEvents|EnhancedInputActionIA_Grapple
  (params (ActionValue :type Boolean) (ElapsedSeconds :type Float%20%28double-precision%29) (TriggeredSeconds :type Float%20%28double-precision%29) (InputAction :type Input%20Action%20Object%20Reference :default "/Game/CatBoomerShooter/Player/Input/IA_Grapple.IA_Grapple"))
  (:Started
    (if (Utilities|Enum|Equal(Enum) (Variables|Default|GetGrappleState) "NewEnumerator0")
      (CallFunction|AttemptGrapple)
      (else
        (CallFunction|CancelGrapple)))))

(event Input|EnhancedActionEvents|EnhancedInputActionIA_Jump
  (params (ActionValue :type Boolean) (ElapsedSeconds :type Float%20%28double-precision%29) (TriggeredSeconds :type Float%20%28double-precision%29) (InputAction :type Input%20Action%20Object%20Reference :default "/Game/CatBoomerShooter/Player/Input/IA_Jump.IA_Jump"))
  (:Started
    (CallFunction|CancelGrapple)))

(event EventTick
  (params (DeltaSeconds :type Float%20%28single-precision%29))
  (Utilities|FlowControl|Sequence
    (:then_0
      (switch Utilities|FlowControl|Switch|SwitchonE_GrappleState (Variables|Default|GetGrappleState)
        (:NewEnumerator0
          (CallFunction|Inactive))
        (:NewEnumerator1
          (CallFunction|Firing))
        (:NewEnumerator2
          (CallFunction|NearTarget))
        (:NewEnumerator3
          (CallFunction|HitTarget))))
    (:then_1
      (Development|PrintString (Utilities|String|Append "GrappleSpeed: " (Utilities|String|ToString(Float) (Variables|Default|GetCurrGrappleSpeed))) true false "(R=0.000000,G=0.660000,B=1.000000,A=1.000000)" 2.0 "GrappleSpeed"))))

(fn SetCurrentTarget
  (params (NewTarget :type BP%20Grapple%20Hook%20Target%20Object%20Reference))
  (if (!= NewTarget (Variables|Default|GetCurrent%20Target))
    (Utilities|FlowControl|Sequence ; Hide  the old Target, Set the New Target and Make the New Target Visible.
      (:then_0
        ;[1 0.7518 0.2891] Hide Old Target
        (bind _current_target (Variables|Default|GetCurrent%20Target)
          (:then
            (Default|SetActive _current_target false))
          (:else)))
      (:then_1
        ;[0.5595 1 0.4855] Set New Target
        (Variables|Default|SetCurrent%20Target NewTarget))
      (:then_2
        ;[0.4214 0.775 1] Show New Target
        (bind _current_target_2 (Variables|Default|GetCurrent%20Target)
          (:then
            (Default|SetActive _current_target_2 true))
          (:else))))))

(fn FindBestTarget
  (params (Targets :type Array%20of%20Actor%20Object%20References))
  (bind _returnvalue (Components|GetOwner))
  (bind _returnvalue_2 (Components|GetOwner))
  (for _array_element Targets
    (LocalVariables|SetCurrentTarget%28Local%29 _array_element)
    (bind _outhit (Collision|LineTraceByChannel (Transformation|GetActorLocation _returnvalue) (Transformation|GetActorLocation (LocalVariables|GetCurrentTarget%28Local%29)) "TraceTypeQuery1" false (Utilities|Array|MakeArray _returnvalue) "None" true "(R=1.000000,G=0.000000,B=0.000000,A=1.000000)" "(R=0.000000,G=1.000000,B=0.000000,A=1.000000)" 0.5))
    (if (== (.HitActor (Collision|BreakHitResult _outhit)) (LocalVariables|GetCurrentTarget%28Local%29))
      (Utilities|FlowControl|Sequence
        (:then_0
          ;[0.1886 0.3492 1] Calculate Angle to Target
          (LocalVariables|SetCurrentAngle%28Local%29 (Class|KismetMathLibrary|DegAcos (Math|Vector|DotProduct (Math|Vector|Normalize (- (Transformation|GetActorLocation (LocalVariables|GetCurrentTarget%28Local%29)) (Transformation|GetActorLocation _returnvalue_2))) (Math|Vector|GetForwardVector (Actor|GetComponentbyClass _returnvalue_2 "/Script/Engine.CameraComponent"))))))
        (:then_1
          ;[1 0.2531 0.8767] Compare the Current Angle to the Best Angle.If the Angle is Less than the Current Angle, or there is No Best Target, make this the Next Target.
          (if (or (< (LocalVariables|GetCurrentAngle%28Local%29) (LocalVariables|GetBestAngle%28Local%29)) (not (Utilities|IsValid (LocalVariables|GetBestTarget%28Local%29))))
            (LocalVariables|SetBestTarget%28Local%29 (LocalVariables|GetCurrentTarget%28Local%29))
            (LocalVariables|SetBestAngle%28Local%29 (LocalVariables|GetCurrentAngle%28Local%29)))))))
  (return (LocalVariables|GetBestTarget%28Local%29)))

(fn HitTarget
  (bind _returnvalue (Components|GetOwner))
  (bind _current_target (Variables|Default|GetCurrent%20Target))
  (bind _returnvalue_2 (Transformation|GetVelocity _returnvalue))
  (bind _returnvalue_3 (/ _returnvalue_2 2.0))
  (bind (_x _y) (Math|Vector|BreakVector _returnvalue_3))
  (if (< (Math|Vector|Distance(Vector) (Transformation|GetActorLocation (Components|GetOwner)) (+ (Transformation|GetActorLocation _current_target) (Variables|/Game/CatBoomerShooter/GrappleHook/BP_GrappleHookTarget.BP_GrappleHookTarget_C|GetCharacterOffset _current_target))) (Variables|Default|GetEndJumpDistance))
    (Utilities|FlowControl|Sequence
      (:then_0
        (Character|LaunchCharacter (.AsCharacter (Utilities|Casting|CastToCharacter _returnvalue)) (Math|Vector|MakeVector _x _y (/ (Variables|Default|GetCurrGrappleSpeed) 1e+01)) true true))
      (:then_1
        (CallFunction|CancelGrapple)))
    (else
      ;[1 0.0542 0.1739] Character Speed to Target
      (bind _output_get (Variables|Default|SetCurrGrappleSpeed (+ (Variables|Default|GetCurrGrappleSpeed) (* (Variables|Default|GetGrappleAccel) (Utilities|Time|GetWorldDeltaSeconds)))))
      (Variables|/Script/Engine.MovementComponent|SetVelocity (Pawn|GetMovementComponent (.AsCharacter (Utilities|Casting|CastToCharacter (Components|GetOwner)))) (* (Utilities|OwnertoTarget) _output_get)))))

(fn NearTarget
  (if (<= (.z (Transformation|GetVelocity (Components|GetOwner))) 0.0)
    (Variables|Default|SetCharacterInitialDirection (Utilities|OwnertoTarget))
    (Variables|Default|SetGrappleState "NewEnumerator3")))

(fn Firing
  (if (< (Default|DistancetoTarget (Variables|Default|GetGrappleHook)) (Variables|Default|GetStartJumpDistance))
    (Character|LaunchCharacter (.AsCharacter (Utilities|Casting|CastToCharacter (Components|GetOwner))) "0.000000,0.000000,500.000000" true true)
    (Variables|Default|SetGrappleState "NewEnumerator2")
    (Variables|Default|SetCurrGrappleSpeed (Variables|Default|GetInitialGrappleSpeed))))

(fn Inactive
  ;[0.5568 0.09369 1] Every Grapple within the Max Distance value can be grappled as a Target.
  (bind _outactors (Collision|SphereOverlapActors (Transformation|GetActorLocation (Components|GetOwner)) (Variables|Default|GetMaxGrappleDistance) (Utilities|Array|MakeArray "ObjectTypeQuery1") "/Game/CatBoomerShooter/GrappleHook/BP_GrappleHookTarget.BP_GrappleHookTarget_C"))
  (bind _target (CallFunction|FindBestTarget _outactors))
  (CallFunction|SetCurrentTarget (.AsBP%20Grapple%20Hook%20Target (Utilities|Casting|CastToBP_GrappleHookTarget _target))))

(fn AttemptGrapple
  (bind _returnvalue (Viewport|GetViewportSize))
  ;[0.5705 1 0.8366] Fire Grapple Hook (View both the Hook and Cable upon Firing)
  (switch Utilities|FlowControl|Switch|SwitchonE_GrappleState (Variables|Default|GetGrappleState)
    (:NewEnumerator0
      (bind _current_target (Variables|Default|GetCurrent%20Target)
        (:then
          (if (Math|Boolean|ANDBoolean (> (.x (.ScreenLocation (Class|PlayerController|ProjectWorldLocationtoScreen (Game|GetPlayerController 0) (Transformation|GetActorLocation _current_target) false))) 0.0) (> (.y (.ScreenLocation (Class|PlayerController|ProjectWorldLocationtoScreen (Game|GetPlayerController 0) (Transformation|GetActorLocation _current_target) false))) 0.0) (< (.x (.ScreenLocation (Class|PlayerController|ProjectWorldLocationtoScreen (Game|GetPlayerController 0) (Transformation|GetActorLocation _current_target) false))) (.x _returnvalue)) (< (.y (.ScreenLocation (Class|PlayerController|ProjectWorldLocationtoScreen (Game|GetPlayerController 0) (Transformation|GetActorLocation _current_target) false))) (.y _returnvalue)))
            (bind _returnvalue_2 (Game|SpawnActorfromClass "/Game/CatBoomerShooter/GrappleHook/BP_GrappleHook.BP_GrappleHook_C" (Math|Transform|MakeTransform (Utilities|OwnerLocation) "0, 0, 0" "1.000000,1.000000,1.000000") "AlwaysSpawn" "MultiplyWithRoot" 0 _current_target 5e+03 0))
            (Variables|Default|SetGrappleHook _returnvalue_2)
            (bind _returnvalue_3 (Game|SpawnActorfromClass "/Game/CatBoomerShooter/GrappleHook/BP_GrappleHookCable.BP_GrappleHookCable_C" (Math|Transform|MakeTransform (Utilities|OwnerLocation) "0, 0, 0" "1.000000,1.000000,1.000000") "AlwaysSpawn" "MultiplyWithRoot" 0 0))
            (bind _output_get (Variables|Default|SetGrappleCable _returnvalue_3))
            (Transformation|AttachComponentToComponent _output_get (Variables|/Script/Engine.Character|GetMesh (.AsCharacter (Utilities|Casting|CastToCharacter (Components|GetOwner)))) (Variables|Default|GetAttachmentSocket) "SnapToTarget" "SnapToTarget" "SnapToTarget" true) ; Attach Grapple Hook and Cable to Player.
            (Class|CableComponent|SetAttachEndto (Variables|/Script/CableComponent.CableActor|GetCableComponent (Variables|Default|GetGrappleCable)) (Variables|Default|GetGrappleHook) "StaticMesh" "None")
            (Transformation|SetActorRotation (Components|GetOwner) (Math|Rotator|MakeRotfromZX (Math|Vector|MakeVector 0.0 0.0 1.0) (Utilities|OwnertoTarget))) ; Set Character to rotate to face the target upon grappling.
            (Variables|Default|SetGrappleState "NewEnumerator1")
            (CallFunction|ToggleGrapplePlayerAnim)))
        (:else)))))

(fn CancelGrapple
  (if (Utilities|Enum|NotEqual(Enum) (Variables|Default|GetGrappleState) "NewEnumerator0")
    (CallFunction|SetCurrentTarget)
    (Actor|DestroyActor (Variables|Default|GetGrappleCable))
    (Variables|Default|SetGrappleCable 0)
    (Actor|DestroyActor (Variables|Default|GetGrappleHook))
    (Variables|Default|SetGrappleHook 0)
    (Variables|Default|SetGrappleState "NewEnumerator0")
    (Variables|Default|SetCurrGrappleSpeed 0.0)
    (CallFunction|ToggleGrapplePlayerAnim)))

(fn ToggleGrapplePlayerAnim
  (bind _asbase_player_character (Utilities|Casting|CastToBasePlayerCharacter (Components|GetOwner)))
  (bind _asabp_fps_arms (Utilities|Casting|CastToABP_FPS_Arms (Components|SkeletalMesh|GetAnimInstance (Variables|/Script/Engine.Character|GetMesh _asbase_player_character))))
  (Variables|/Game/CatBoomerShooter/Characters/Player/ABP_FPS_Arms.ABP_FPS_Arms_C|SetShowGrapple _asabp_fps_arms (Utilities|Enum|NotEqual(Enum) (Variables|Default|GetGrappleState) "NewEnumerator0")))