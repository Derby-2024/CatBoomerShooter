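; Grapple hook rope visual that attaches to the owning player's left hand socket and extends toward a target location.
; Each tick it advances the rope tip at a set speed, then clears and rebuilds the rope.
; A near-zero-gravity projectile prediction, traced from the tip back toward the hand against pawns, supplies the spline points.
; Spline meshes span each segment, with instanced meshes oriented along the spline at interior points.
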(event EventBeginPlay
  (bind _asbase_player_character (Utilities|Casting|CastToBasePlayerCharacter (Components|GetOwner)))
  (Transformation|AttachComponentToComponent (Variables|/Script/Engine.Character|GetMesh _asbase_player_character) "L_HandSocket" "SnapToTarget" "SnapToTarget" "SnapToTarget" true)
  (bind _returnvalue (AddComponent|AddSplineComponent false))
  (Variables|Default|SetSplineComp _returnvalue)
  (bind _returnvalue_2 (AddComponent|AddInstancedStaticMeshComponent true))
  (Variables|Default|SetInstancedStaticMesh _returnvalue_2)
  (Variables|Default|SetCurrTargetLocation (Transformation|GetActorLocation)))

(event EventTick
  (params (DeltaSeconds :type Float%20%28single-precision%29))
  (Utilities|FlowControl|Sequence
    (:then_0
      (if (Utilities|Operators|NotEqual(!=) (Variables|Default|GetCurrTargetLocation) (Variables|Default|GetTargetLocation) 5.0)
        (Variables|Default|SetCurrTargetLocation (+ (* (Math|Vector|GetUnitDirection(Vector) (Variables|Default|GetCurrTargetLocation) (Variables|Default|GetTargetLocation)) (Variables|Default|GetSpeed) DeltaSeconds) (Variables|Default|GetCurrTargetLocation)))))
    (:then_1
      (CallFunction|UpdateSpline))))

(fn ConstructionScript)

(fn UpdateSpline
  (bind _currtargetlocation (Variables|Default|GetCurrTargetLocation))
  (bind _splinecomp (Variables|Default|GetSplineComp))
  (CallFunction|ClearSpline)
  (bind _predictresult (Class|GameplayStatics|BlueprintPredictProjectilePathAdvanced (Utilities|Struct|MakePredictProjectilePathParams _currtargetlocation (* (Math|Vector|GetUnitDirection(Vector) _currtargetlocation (Transformation|GetActorLocation)) 1.5e+03) true 0.0 5.0 true "ECC_Pawn" (Utilities|Array|MakeArray "ObjectTypeQuery3") 0 2e+01 -1.0 "None" 1.0 false)))
  (bind _array_element (Utilities|Array|ForEachLoopwithBreak (.PathData (Utilities|Struct|BreakPredictProjectilePathResult _predictresult)))
    (:LoopBody
      (Spline|AddSplinePoint (Variables|Default|GetSplineComp) (.Location (Utilities|Struct|BreakPredictProjectilePathPointData _array_element)) "World" true))
    (:Completed
      (for _index (range 0 (- (Spline|GetNumberOfSplinePoints (Variables|Default|GetSplineComp)) 2))
        (bind _returnvalue (AddComponent|AddSplineMeshComponent true))
        (Utilities|Array|Add (Variables|Default|GetSplineMeshComps) _returnvalue)
        (SplineMesh|SetStartandEnd _returnvalue (.Location (Spline|GetLocationandTangentatSplinePoint _splinecomp _index "World")) (.Tangent (Spline|GetLocationandTangentatSplinePoint _splinecomp _index "World")) (.Location (Spline|GetLocationandTangentatSplinePoint _splinecomp (+ _index 1) "World")) (.Tangent (Spline|GetLocationandTangentatSplinePoint _splinecomp (+ _index 1) "World")) true :!class /Script/Engine.SplineMeshComponent)
        (if (> _index 0)
          (Components|InstancedStaticMesh|AddInstance (Variables|Default|GetInstancedStaticMesh) (Math|Transform|MakeTransform (.Location (Spline|GetLocationandTangentatSplinePoint _splinecomp _index "World")) (Math|Rotator|MakeRotfromX (Class|SplineComponent|GetDirectionatSplinePoint _splinecomp _index "World")) "1.000000,1.000000,1.000000") true))))))

(fn ClearSpline
  (bind _splinekeymeshes (Variables|Default|GetSplineKeyMeshes))
  (bind _splinemeshcomps (Variables|Default|GetSplineMeshComps))
  (Components|InstancedStaticMesh|ClearInstances (Variables|Default|GetInstancedStaticMesh))
  (Components|DestroyComponent _splinemeshcomps)
  (Components|DestroyComponent _splinekeymeshes)
  (Utilities|Array|Clear _splinekeymeshes)
  (Utilities|Array|Clear _splinemeshcomps)
  (Spline|ClearSplinePoints (Variables|Default|GetSplineComp) true))

(fn DistancetoTarget
  (return (Math|Vector|Distance(Vector) (Variables|Default|GetCurrTargetLocation) (Variables|Default|GetTargetLocation))))