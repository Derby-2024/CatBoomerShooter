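; AI controller for the tank grenade enemy that turns perception stimuli into blackboard state for its behaviour.
; Perception updates are routed by sense to sight, hearing and damage handlers, which set the state enum and AttackTarget.
; Losing sight switches to another state and stores LastKnownLocation.
; Active sight takes priority: hearing and damage only set the target while nothing is seen.
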(event OnTargetPerceptionUpdated(AIPerception)
  (params (Actor :type Actor%20Object%20Reference) (Stimulus :type AI%20Stimulus%20Structure))
  (bind _returnvalue (Class|AIPerceptionSystem|GetSenseClassforStimulus Stimulus))
  (if (== _returnvalue "/Script/AIModule.AISense_Sight")
    (CallFunction|HandleSight Actor Stimulus)
    (elif (== _returnvalue "/Script/AIModule.AISense_Hearing")
      (CallFunction|HandleHearing Actor Stimulus)
      (elif (== _returnvalue "/Script/AIModule.AISense_Damage")
        (CallFunction|HandleDamage Actor Stimulus)))))

(fn ConstructionScript)

(fn HandleSight
  (params (SensedActor :type Actor%20Object%20Reference) (SightStimulus :type AI%20Stimulus%20Structure))
  (if (.bsuccessfullysensed SightStimulus)
    (Variables|Default|SetIsSightActive true)
    (AI|Components|Blackboard|SetValueasEnum (AI|GetBlackboard 0) (Variables|Default|GetStateKeyName) (Utilities|Enum|LiteralenumE_BehaviourStates "NewEnumerator1"))
    (AI|Components|Blackboard|SetValueasObject (AI|GetBlackboard 0) (Utilities|Name|MakeLiteralName "AttackTarget") SensedActor)
    (else
      (Variables|Default|SetIsSightActive false)
      (AI|Components|Blackboard|SetValueasEnum (AI|GetBlackboard 0) (Variables|Default|GetStateKeyName) (Utilities|Enum|LiteralenumE_BehaviourStates "NewEnumerator3"))
      (AI|Components|Blackboard|SetValueasVector (AI|GetBlackboard 0) (Utilities|Name|MakeLiteralName "LastKnownLocation") (.stimuluslocation SightStimulus))))
  (return))

(fn HandleHearing
  (params (SensedActor :type Actor%20Object%20Reference) (HearingStimulus :type AI%20Stimulus%20Structure))
  (if (.bsuccessfullysensed HearingStimulus)
    (if (Variables|Default|GetIsSightActive)
      _
      (else
        (AI|Components|Blackboard|SetValueasEnum (AI|GetBlackboard 0) (Variables|Default|GetStateKeyName) (Utilities|Enum|LiteralenumE_BehaviourStates "NewEnumerator1"))
        (AI|Components|Blackboard|SetValueasObject (AI|GetBlackboard 0) (Utilities|Name|MakeLiteralName "AttackTarget") SensedActor))))
  (return))

(fn HandleDamage
  (params (SensedActor :type Actor%20Object%20Reference) (DamageStimulus :type AI%20Stimulus%20Structure))
  (if (.bsuccessfullysensed DamageStimulus)
    (if (Variables|Default|GetIsSightActive)
      _
      (else
        (AI|Components|Blackboard|SetValueasEnum (AI|GetBlackboard 0) (Variables|Default|GetStateKeyName) (Utilities|Enum|LiteralenumE_BehaviourStates "NewEnumerator1"))
        (AI|Components|Blackboard|SetValueasObject (AI|GetBlackboard 0) (Utilities|Name|MakeLiteralName "AttackTarget") SensedActor))))
  (return))