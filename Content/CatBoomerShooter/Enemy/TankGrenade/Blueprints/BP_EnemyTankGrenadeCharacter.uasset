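; Armoured enemy tank character that fires grenades from a spawn point and exposes a patrol route and selectable walk speed.
; Damage drains armour before health, and the enemy is destroyed when a hit would push health below zero.
; As armour falls to successive thresholds, it hides the matching armour mesh piece, at most one per hit, and prints debug stats.
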(event Custom|ShootWeapon
  ;[0 0.0836 1] Shoot Weapon
  (Game|SpawnActorfromClass "/Game/CatBoomerShooter/Enemy/TankGrenade/Blueprints/BP_Grenade.BP_Grenade_C" (Transformation|GetWorldTransform (Variables|Default|GetGrenadeSpawnLocation)) "Undefined" "MultiplyWithRoot" self 0))

(event Custom|DamageHealth
  (params (DamageAmount :type Float%20%28double-precision%29))
  (bind _self self)
  (bind _returnvalue (Utilities|GetDisplayName _self))
  ;[1 0 0] Damage the Tank
  (if (< (- (Variables|Default|GetHealth) DamageAmount) 0.0)
    (bind _output_get (Variables|Default|SetHealth 0.0))
    (bind _output_get_2 (Variables|Default|SetHealthRemaining (Utilities|String|ToString(Float) _output_get)))
    (Development|PrintString (Utilities|String|Append _returnvalue ".HEALTH: " _output_get_2) true true "(R=1.000000,G=0.011765,B=0.000000,A=1.000000)")
    (Actor|DestroyActor)
    (else
      (bind _output_get_3 (Variables|Default|SetHealth (- (Variables|Default|GetHealth) DamageAmount)))
      (bind _output_get_4 (Variables|Default|SetHealthRemaining (Utilities|String|ToString(Float) _output_get_3)))
      (Development|PrintString (Utilities|String|Append _returnvalue ".HEALTH: " _output_get_4) true true "(R=1.000000,G=0.011765,B=0.000000,A=1.000000)"))))

(event Custom|DamageArmour
  (params (DamageAmount :type Float%20%28double-precision%29))
  (bind _self self)
  (bind _returnvalue (Utilities|GetDisplayName _self))
  ;[1 0 0] Damage the Tank
  (if (< (- (Variables|Default|GetArmour) DamageAmount) 0.0)
    (Variables|Default|SetArmour 0.0)
    (else
      (Variables|Default|SetArmour (- (Variables|Default|GetArmour) DamageAmount))))
  (if (> (Variables|Default|GetArmour) (Utilities|Array|Get(acopy) (Variables|Default|GetArmourThresholds) (Variables|Default|GetArmourThresholdsIndex)))
    (bind _output_get (Variables|Default|SetArmourRemaining "" :!label _label))
    (Development|PrintString (Utilities|String|Append _returnvalue ".ARMOUR: " _output_get) true true "(R=0.219608,G=0.164706,B=0.168627,A=1.000000)")
    (else
      (bind _output_get_2 (Variables|Default|SetArmourPiecesIndex (Variables|Default|GetArmourThresholdsIndex)))
      (Rendering|SetVisibility (Utilities|Array|Get(acopy) (Variables|Default|GetArmourPieces) _output_get_2) false false)
      (if (>= (Variables|Default|GetArmourThresholdsIndex) (- (Utilities|Array|Length (Variables|Default|GetArmourThresholds)) 1))
        (Variables|Default|SetArmourThresholdsIndex 0)
        (else
          (bind _result (Math|Integer|IncrementInt (Variables|Default|GetArmourThresholdsIndex))
            (:%20%20
              (Variables|Default|SetArmourThresholdsIndex _result)))))
      (if (< (Variables|Default|GetArmour) 0.0)
        (bind _output_get_3 (Variables|Default|SetArmourRemaining ""))
        (Development|PrintString (Utilities|String|Append _returnvalue ".ARMOUR: " _output_get_3) true true "(R=0.219608,G=0.164706,B=0.168627,A=1.000000)")
        (Utilities|Array|Clear (Variables|Default|GetArmourPieces))
        (else
          (goto _label))))))

(event Game|Damage|EventAnyDamage
  (params (Damage :type Float%20%28single-precision%29) (DamageType :type Damage%20Type%20Object%20Reference) (InstigatedBy :type Controller%20Object%20Reference) (DamageCauser :type Actor%20Object%20Reference))
  ;[1 0 0] Damage the Tank
  (if (<= (Variables|Default|GetArmour) 0.0)
    (CallFunction|DamageHealth Damage)
    (else
      (CallFunction|DamageArmour Damage))))

(event EventBeginPlay
  ;[1 1 1] Begin Play
  (Variables|Default|SetArmourPieces (Utilities|Array|MakeArray (Variables|Default|GetArmourArmRight) (Variables|Default|GetArmourArmLeft) (Variables|Default|GetArmourLegRight) (Variables|Default|GetArmourLegLeft) (Variables|Default|GetArmourHelmet) (Variables|Default|GetArmourChest))))

(fn ConstructionScript)

(fn GetPatrolRoute
  (return (Variables|Default|GetPatrolRoute)))

(fn SetMovementSpeed
  (params (MovementSpeed :type E_MovementSpeeds%20Enum :default "NewEnumerator0"))
  (bind _output_get (Variables|/Script/Engine.CharacterMovementComponent|SetMaxWalkSpeed (Variables|Character|GetCharacterMovement) (Utilities|Select :Index MovementSpeed :NewEnumerator0 1e+02 :NewEnumerator1 3e+02)))
  (return _output_get))