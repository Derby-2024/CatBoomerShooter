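; Bomber enemy Character that carries a bomb and explodes, dealing radial damage with a physics impulse before destroying itself.
; Lethal damage, or a Body hit or overlap while Health exceeds 1, destroys the Body, releases the Bomb to physics and starts Boom.
; Boom waits on a shared Delay variable, which Bomb impacts zero and low-health Body contacts lengthen without detonating.
; Updatespeed exposes walk speed control.
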(event OnComponentHit(Bomb)
  (params (HitComponent :type Primitive%20Component%20Object%20Reference) (OtherActor :type Actor%20Object%20Reference) (OtherComp :type Primitive%20Component%20Object%20Reference) (NormalImpulse :type Vector :default "0, 0, 0") (Hit :type Hit%20Result%20Structure%20%28by%20ref%29))
  (Development|PrintString "bomb hit")
  (Variables|Default|SetDelay 0.0)
  (CallFunction|Boom))

(event OnComponentHit(Body)
  (params (HitComponent :type Primitive%20Component%20Object%20Reference) (OtherActor :type Actor%20Object%20Reference) (OtherComp :type Primitive%20Component%20Object%20Reference) (NormalImpulse :type Vector :default "0, 0, 0") (Hit :type Hit%20Result%20Structure%20%28by%20ref%29))
  (Development|PrintString "Hit")
  (if (> (Variables|Default|GetHealth) 1)
    (Variables|Default|SetHealth (- (Variables|Default|GetHealth) 1))
    (Components|DestroyComponent (Variables|Default|GetBody))
    (Physics|SetSimulatePhysics (Variables|Default|GetBomb) true)
    (CallFunction|Boom)
    (else
      (Variables|Default|SetDelay 3.0))))

(event OnComponentBeginOverlap(Body)
  (params (OverlappedComponent :type Primitive%20Component%20Object%20Reference) (OtherActor :type Actor%20Object%20Reference) (OtherComp :type Primitive%20Component%20Object%20Reference) (OtherBodyIndex :type Integer) (bFromSweep :type Boolean) (SweepResult :type Hit%20Result%20Structure%20%28by%20ref%29))
  (Development|PrintString "Hit")
  (if (> (Variables|Default|GetHealth) 1)
    (Variables|Default|SetHealth (- (Variables|Default|GetHealth) 1))
    (Components|DestroyComponent (Variables|Default|GetBody))
    (Physics|SetSimulatePhysics (Variables|Default|GetBomb) true)
    (CallFunction|Boom)
    (else
      (Variables|Default|SetDelay 3.0))))

(event Custom|Boom
  (bind _bomb (Variables|Default|GetBomb))
  (bind _returnvalue (Transformation|GetWorldLocation _bomb))
  (Utilities|FlowControl|Delay (Variables|Default|GetDelay))
  (Effects|SpawnEmitteratLocation 0 _returnvalue)
  (Audio|PlaySoundatLocation 0 _returnvalue "0, 0, 0" 1.0 1.0 0.0 0 0 0 0)
  (Game|Damage|ApplyRadialDamage 5.0 _returnvalue 3e+02 0 0 0 0 true "ECC_Visibility")
  (Class|RadialForceComponent|FireImpulse (Variables|Default|Getexplosive%20force))
  (Actor|DestroyActor))

(event EventBeginPlay)

(event Collision|EventActorBeginOverlap
  (params (OtherActor :type Actor%20Object%20Reference)))

(event EventTick
  (params (DeltaSeconds :type Float%20%28single-precision%29)))

(event Game|Damage|EventAnyDamage
  (params (Damage :type Float%20%28single-precision%29) (DamageType :type Damage%20Type%20Object%20Reference) (InstigatedBy :type Controller%20Object%20Reference) (DamageCauser :type Actor%20Object%20Reference))
  (Variables|Default|SetHealth (- (Variables|Default|GetHealth) Damage))
  (Development|PrintString "damage " true true "(R=0.095132,G=1.000000,B=0.000000,A=1.000000)")
  (if (not (> (Variables|Default|GetHealth) 0.0))
    (Components|DestroyComponent (Variables|Default|GetBody))
    (Physics|SetSimulatePhysics (Variables|Default|GetBomb) true)
    (CallFunction|Boom)))

(fn ConstructionScript)

(fn Updatespeed
  (params (New%20speed :type Float%20%28double-precision%29))
  (Variables|/Script/Engine.CharacterMovementComponent|SetMaxWalkSpeed (Variables|Character|GetCharacterMovement) New%20speed))