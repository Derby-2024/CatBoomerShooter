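; BP_Enemy is an enemy with a health value and a world-space health bar widget.
; Every tick it pushes Health, scaled from a 100-point range, into the WBP_EnemyHealth slider and rotates the bar to face the player character.
; In the same tick it destroys itself once Health drops to zero or below.
; The file holds no damage, movement or AI logic.
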(event Collision|EventActorBeginOverlap
  (params (OtherActor :type Actor%20Object%20Reference)))

(event EventTick
  (params (DeltaSeconds :type Float%20%28single-precision%29))
  (Utilities|FlowControl|Sequence
    (:then_0
      (bind _aswbp_enemy_health (Utilities|Casting|CastToWBP_EnemyHealth (UserInterface|GetWidget (Variables|Default|GetHealthBar))))
      (Progress|SetPercent (Variables|/Game/CatBoomerShooter/Enemy/WBP_EnemyHealth.WBP_EnemyHealth_C|GetHealthSlider _aswbp_enemy_health) (/ (Variables|Default|GetHealth) 1e+02))
      (Transformation|SetWorldRotation (Variables|Default|GetHealthBar) (Math|Rotator|FindLookatRotation (Transformation|GetWorldLocation (Variables|Default|GetHealthBar)) (Transformation|GetActorLocation (Game|GetPlayerCharacter 0))) false false))
    (:then_1
      (if (<= (Variables|Default|GetHealth) 0.0)
        (Actor|DestroyActor)))))

(event EventBeginPlay)

(fn ConstructionScript)