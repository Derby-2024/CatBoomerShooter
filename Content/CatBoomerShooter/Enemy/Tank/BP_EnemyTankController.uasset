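; AI controller for the tank enemy that runs the BT_EnemyTank behavior tree on BeginPlay.
; Perception updates pass to HandleSight, which only reacts to actors tagged Player.
; A successful sighting sets CanSeePlayer and stores the SpottedActor on the blackboard; losing sight clears both, with debug prints for each case.
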(event OnTargetPerceptionUpdated(AIPerception)
  (params (Actor :type Actor%20Object%20Reference) (Stimulus :type AI%20Stimulus%20Structure))
  (Utilities|FlowControl|Sequence
    (:then_0
      (CallFunction|HandleSight Actor Stimulus))))

(event EventBeginPlay
  (AI|RunBehaviorTree "/Game/CatBoomerShooter/Enemy/Tank/BT_EnemyTank.BT_EnemyTank"))

(fn ConstructionScript)

(fn HandleSight
  (params (SensedActor :type Actor%20Object%20Reference) (SightStimulus :type AI%20Stimulus%20Structure))
  (if (Actor|ActorHasTag SensedActor "Player")
    (if (.bsuccessfullysensed SightStimulus)
      (Development|PrintString "Target Seen!")
      (AI|Components|Blackboard|SetValueasBool (AI|GetBlackboard 0) (Utilities|Name|MakeLiteralName "CanSeePlayer") true)
      (AI|Components|Blackboard|SetValueasObject (AI|GetBlackboard 0) (Utilities|Name|MakeLiteralName "SpottedActor") SensedActor)
      (else
        (Development|PrintString "Moving to Player...")
        (AI|Components|Blackboard|SetValueasBool (AI|GetBlackboard 0) (Utilities|Name|MakeLiteralName "CanSeePlayer") false)
        (AI|Components|Blackboard|SetValueasObject (AI|GetBlackboard 0) (Utilities|Name|MakeLiteralName "SpottedActor") 0)))))