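; AI controller for the tank enemy that turns perception updates into Blackboard data.
; Every target perception update goes straight to HandleSight without checking sense type or actor class.
; A successful sense switches the E_States state and stores the actor as AttackTarget.
; A lost sense switches to another state and saves the stimulus location as LastKnownLocation, with debug prints in both cases.
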(event OnTargetPerceptionUpdated(AIPerception)
  (params (Actor :type Actor%20Object%20Reference) (Stimulus :type AI%20Stimulus%20Structure))
  (Utilities|FlowControl|Sequence
    (:then_0
      (CallFunction|HandleSight Actor Stimulus))))

(fn ConstructionScript)

(fn HandleSight
  (params (SensedActor :type Actor%20Object%20Reference) (SightStimulus :type AI%20Stimulus%20Structure))
  (if (.bsuccessfullysensed SightStimulus)
    (Development|PrintString "Target Seen!")
    (AI|Components|Blackboard|SetValueasEnum (AI|GetBlackboard 0) (Variables|Default|GetStateKeyName) (Utilities|Enum|LiteralenumE_States "NewEnumerator1"))
    (AI|Components|Blackboard|SetValueasObject (AI|GetBlackboard 0) (Utilities|Name|MakeLiteralName "AttackTarget") SensedActor)
    (else
      (Development|PrintString "Lost Target!")
      (AI|Components|Blackboard|SetValueasEnum (AI|GetBlackboard 0) (Variables|Default|GetStateKeyName) (Utilities|Enum|LiteralenumE_States "NewEnumerator3"))
      (AI|Components|Blackboard|SetValueasVector (AI|GetBlackboard 0) (Utilities|Name|MakeLiteralName "LastKnownLocation") (.stimuluslocation SightStimulus)))))