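; Tank enemy character for the shooter, with armour, health, a patrol route and selectable walk speed.
; Incoming damage drains armour before health without carrying overflow across, prints debug values, and destroys the actor when health would drop below zero.
; ShootWeapon line-traces to the target on the Camera channel but deals no damage yet; random damage and accuracy nodes sit unused.
; GetPatrolRoute and SetMovementSpeed expose the route and min/max speed switching.
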(event Custom|DamageHealth
  (params (DamageAmount :type Float%20%28double-precision%29))
  ;[1 1 1] Damage the Enemy
  (if (< (- (Variables|Default|GetHealth) DamageAmount) 0.0)
    (bind _output_get (Variables|Default|SetHealth 0.0))
    (Variables|Default|SetHealthRemaining (Utilities|String|ToString(Float) _output_get))
    (Development|PrintString (Utilities|String|Append "HEALTH:  " ""))
    (Actor|DestroyActor)
    (else
      (bind _output_get_2 (Variables|Default|SetHealth (- (Variables|Default|GetHealth) DamageAmount)))
      (bind _output_get_3 (Variables|Default|SetHealthRemaining (Utilities|String|ToString(Float) _output_get_2)))
      (Development|PrintString (Utilities|String|Append "HEALTH:  " _output_get_3)))))

(event Custom|ShootWeapon
  (params (AttackTarget :type Actor%20Object%20Reference))
  ;[1 1 1] Shoot the Player
  (if (Utilities|IsValid AttackTarget)
    (bind (_outhit _returnvalue) (Collision|LineTraceByChannel (Transformation|GetActorLocation) (Transformation|GetActorLocation AttackTarget) "TraceTypeQuery2" false 0 "None"))
    (if _returnvalue
      (if (== AttackTarget (.HitActor (Collision|BreakHitResult _outhit)))
        _))))

(event Custom|DamageArmour
  (params (DamageAmount :type Float%20%28double-precision%29))
  ;[1 1 1] Damage the Enemy
  (if (< (- (Variables|Default|GetArmour) DamageAmount) 0.0)
    (bind _output_get (Variables|Default|SetArmour 0.0))
    (bind _output_get_2 (Variables|Default|SetArmourRemaining (Utilities|String|ToString(Float) _output_get)))
    (Development|PrintString (Utilities|String|Append "ARMOUR:  " _output_get_2))
    (else
      (bind _output_get_3 (Variables|Default|SetArmour (- (Variables|Default|GetArmour) DamageAmount)))
      (bind _output_get_4 (Variables|Default|SetArmourRemaining (Utilities|String|ToString(Float) _output_get_3)))
      (Development|PrintString (Utilities|String|Append "ARMOUR:  " _output_get_4)))))

(event Game|Damage|EventAnyDamage
  (params (Damage :type Float%20%28single-precision%29) (DamageType :type Damage%20Type%20Object%20Reference) (InstigatedBy :type Controller%20Object%20Reference) (DamageCauser :type Actor%20Object%20Reference))
  ;[1 1 1] Damage the Enemy
  (if (<= (Variables|Default|GetArmour) 0.0)
    (CallFunction|DamageHealth Damage)
    (else
      (CallFunction|DamageArmour Damage))))

(fn ConstructionScript)

(fn GetPatrolRoute
  (return (Variables|Default|GetPatrolRoute)))

(fn SetMovementSpeed
  (params (Speed :type E_MovementSpeeds%20Enum :default "NewEnumerator0"))
  (bind _output_get (Variables|/Script/Engine.CharacterMovementComponent|SetMaxWalkSpeed (Variables|Character|GetCharacterMovement) (Utilities|Select :Index Speed :NewEnumerator0 1e+02 :NewEnumerator1 3e+02)))
  (return _output_get))