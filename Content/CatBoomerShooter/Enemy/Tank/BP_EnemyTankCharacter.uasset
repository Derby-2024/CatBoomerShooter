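; BP_EnemyTankCharacter is the tank enemy character, providing a hitscan weapon attack against a target player.
; ShootWeapon line-traces on the Camera channel from the tank's location to a valid target's location.
; If the trace hits that player, it sends a TakeDamage message with random damage between the weapon's minimum and maximum.
; An accuracy offset based on WeaponAccuracy is left unconnected, so shots have no spread.
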(event Custom|ShootWeapon
  (params (TargetPlayer :type Actor%20Object%20Reference))
  (if (Utilities|IsValid TargetPlayer)
    (bind (_outhit _returnvalue) (Collision|LineTraceByChannel (Transformation|GetActorLocation) (Transformation|GetActorLocation TargetPlayer) "TraceTypeQuery2" false 0 "None"))
    (if _returnvalue
      (if (== TargetPlayer (.HitActor (Collision|BreakHitResult _outhit)))
        (Class|BITakeDamage|TakeDamage(Message) (.HitActor (Collision|BreakHitResult _outhit)) (Math|Random|RandomFloatinRange (Variables|Default|GetWeaponMinDamage) (Variables|Default|GetWeaponMaxDamage)))))))

(fn ConstructionScript)