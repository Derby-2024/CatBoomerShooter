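; BP_Mortar is a mortar attack marker, filed under the boss cat mech's custom attacks, that telegraphs an impact zone.
; On BeginPlay it starts a warning timer, traces downward to find the surface and draws a debug cylinder there for the warning's duration.
; When the timer fires, the actor destroys itself and draws a debug sphere at its own location, with no damage applied.
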(event Custom|Fire
  (Actor|DestroyActor)
  (Rendering|Debug|DrawDebugSphere (Transformation|GetActorLocation) 2e+02 12 "(R=1.000000,G=0.000000,B=0.123857,A=1.000000)" 2.0 2e+01))

(event EventBeginPlay
  (bind _returnvalue (Transformation|GetActorLocation))
  (Utilities|Time|SetTimerbyEvent (delegate Custom|Fire) (Variables|Default|GetWarningTime))
  (bind _outhit (Collision|LineTraceByChannel _returnvalue (+ _returnvalue (* (Transformation|GetActorUpVector) -3e+02)) "TraceTypeQuery1" false 0 "None"))
  (Class|KismetSystemLibrary|DrawDebugCylinder (.Location (Collision|BreakHitResult _outhit)) (.Location (Collision|BreakHitResult _outhit)) 2e+02 12 "(R=0.976175,G=0.039800,B=1.000000,A=1.000000)" (Variables|Default|GetWarningTime) 2e+01))

(fn ConstructionScript)