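; Base weapon pickup that gives the player a configured weapon, or ammo if they already own it.
; Sphere overlap adds ammo of the matching weapon's type to the inventory, or adds and equips the weapon on player and HUD.
; Used pickups are hidden with collision off rather than destroyed, and ActorLoaded reapplies that disabled state.
; The construction script sets the mesh; BeginPlay destroys pickups lacking a valid class or mesh.
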(event OnComponentBeginOverlap(Sphere)
  (params (OverlappedComponent :type Primitive%20Component%20Object%20Reference) (OtherActor :type Actor%20Object%20Reference) (OtherComp :type Primitive%20Component%20Object%20Reference) (OtherBodyIndex :type Integer) (bFromSweep :type Boolean) (SweepResult :type Hit%20Result%20Structure%20%28by%20ref%29))
  (bind _returnvalue (Game|GetPlayerCharacter 0))
  (if (== OtherActor _returnvalue)
    (bind _asbp_player_character (Utilities|Casting|CastToBP_PlayerCharacter _returnvalue))
    (bind _array_element (Utilities|Array|ForEachLoopwithBreak (Variables|/Script/CatBoomerShooter.BasePlayerCharacter|GetWeaponList _asbp_player_character))
      (:LoopBody
        (if (== (Utilities|GetClass _array_element) (Variables|Default|GetWeaponBlueprint))
          (Class|InventoryComponent|AddItem (Class|BasePlayerCharacter|GetInventoryComponent _asbp_player_character) (Utilities|Struct|MakeItem "Ammo" (Variables|Default|GetAmmoAmount) 0 (Variables|/Script/CatBoomerShooter.BaseWeapon|GetAmmoType _array_element) "" 0 0 "" "E_Cat"))
          (Rendering|SetActorHiddenInGame true)
          (Collision|SetCollisionEnabled (Variables|Default|GetSphere) "NoCollision")
          (Variables|Default|SetIsAmmo true)
          (Variables|Default|SetisDisabled true)))
      (:Completed
        (if (not (Variables|Default|GetIsAmmo))
          (bind _returnvalue_2 (Class|BasePlayerCharacter|AddWeapon _asbp_player_character (Variables|Default|GetWeaponBlueprint)))
          (Default|AddWeapon (Variables|/Game/CatBoomerShooter/Player/BP_PlayerCharacter.BP_PlayerCharacter_C|GetHUD _asbp_player_character) _returnvalue_2)
          (Class|BasePlayerCharacter|EquipWeapon _asbp_player_character _returnvalue_2)
          (Default|EquipWeapon (Variables|/Game/CatBoomerShooter/Player/BP_PlayerCharacter.BP_PlayerCharacter_C|GetHUD _asbp_player_character) _returnvalue_2)
          (Rendering|SetActorHiddenInGame true)
          (Collision|SetCollisionEnabled (Variables|Default|GetSphere) "NoCollision")
          (Variables|Default|SetisDisabled true))))))

(event EventBeginPlay
  (if (Utilities|IsValidClass (Variables|Default|GetWeaponBlueprint))
    (Utilities|IsValid (Components|SkeletalMesh|GetSkeletalMeshAsset (Variables|Default|GetWeaponMesh))
      (:Is%20Not%20Valid
        _)))
  (Actor|DestroyActor))

(event EventActorLoaded
  (CallFunction|CheckActorDisabled))

(fn ConstructionScript
  (Components|SkeletalMesh|SetSkeletalMeshAsset (Variables|Default|GetWeaponMesh) (Variables|Default|GetWeaponSkeletalMesh)))

(fn CheckActorDisabled
  (bind _isdisabled (Variables|Default|GetisDisabled))
  (Rendering|SetActorHiddenInGame _isdisabled)
  (Collision|SetCollisionEnabled (Variables|Default|GetSphere) (select _isdisabled "NoCollision" "QueryOnly")))

(fn ComponentstoSave
  (return 0))