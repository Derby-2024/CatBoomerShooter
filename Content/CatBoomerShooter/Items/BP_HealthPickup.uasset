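; BP_HealthPickup is a health pickup that restores the player's health on contact.
; When its Collision component overlaps a BP_PlayerCharacter below max health, it adds HealthAmount to the HealthComponent's Health, capped at MaxHealth.
; The pickup then destroys itself, while overlaps from a player at full health or from other actors leave it in place.
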(event OnComponentBeginOverlap(Collision)
  (params (OverlappedComponent :type Primitive%20Component%20Object%20Reference) (OtherActor :type Actor%20Object%20Reference) (OtherComp :type Primitive%20Component%20Object%20Reference) (OtherBodyIndex :type Integer) (bFromSweep :type Boolean) (SweepResult :type Hit%20Result%20Structure%20%28by%20ref%29))
  (bind _asbp_player_character (Utilities|Casting|CastToBP_PlayerCharacter OtherActor))
  (if (not (== (Variables|/Script/CatBoomerShooter.HealthComponent|GetMaxHealth (Variables|/Script/CatBoomerShooter.BasePlayerCharacter|GetHealthComponent _asbp_player_character)) (Variables|/Script/CatBoomerShooter.HealthComponent|GetHealth (Variables|/Script/CatBoomerShooter.BasePlayerCharacter|GetHealthComponent _asbp_player_character))))
    (Variables|/Script/CatBoomerShooter.HealthComponent|SetHealth (Variables|/Script/CatBoomerShooter.BasePlayerCharacter|GetHealthComponent _asbp_player_character) (Math|Float|Min(Float) (+ (Variables|/Script/CatBoomerShooter.HealthComponent|GetHealth (Variables|/Script/CatBoomerShooter.BasePlayerCharacter|GetHealthComponent _asbp_player_character)) (Variables|Default|GetHealthAmount)) (Variables|/Script/CatBoomerShooter.HealthComponent|GetMaxHealth (Variables|/Script/CatBoomerShooter.BasePlayerCharacter|GetHealthComponent _asbp_player_character))))
    (Actor|DestroyActor)))

(fn ConstructionScript)