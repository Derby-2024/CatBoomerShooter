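; Armoured tank enemy character that fights with a grenade launcher spawned on BeginPlay and fired through ShootWeapon.
; Incoming damage is reported to AI damage sensing at the player's location, then depletes armour before health.
; Crossed armour thresholds detach physics-simulated pieces and destroy them on a short timer, while zero health destroys character and weapon.
; Helper functions expose the patrol route, per-weapon damage values and walk speed switching.
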(event Custom|ShootWeapon
  ;[0 0.0836 1] Shoot Weapon
  (Class|BaseWeapon|StartShooting (Variables|Default|GetWeapon)))

(event Custom|DamageHealth
  (params (DamageAmount :type Float%20%28double-precision%29) (LeftoverDamage :type Float%20%28double-precision%29))
  (bind _self self)
  (bind _returnvalue (Utilities|GetDisplayName _self))
  ;[1 0 0] Damage the Tank
  (Variables|Default|SetLeftoverDamage 0.0)
  (if (<= (- (Variables|Default|GetHealth) (+ DamageAmount LeftoverDamage)) 0.0)
    (bind _output_get (Variables|Default|SetHealth 0.0))
    (bind _output_get_2 (Variables|Default|SetHealthRemaining (Utilities|String|ToString(Float) _output_get)))
    (Development|PrintString (Utilities|String|Append _returnvalue ".HEALTH: " _output_get_2) true true "(R=1.000000,G=0.011765,B=0.000000,A=1.000000)")
    (Actor|DestroyActor (Variables|Default|GetWeapon))
    (Actor|DestroyActor)
    (else
      (bind _output_get_3 (Variables|Default|SetHealth (- (Variables|Default|GetHealth) (+ DamageAmount LeftoverDamage))))
      (bind _output_get_4 (Variables|Default|SetHealthRemaining (Utilities|String|ToString(Float) _output_get_3)))
      (Development|PrintString (Utilities|String|Append _returnvalue ".HEALTH: " _output_get_4) true true "(R=1.000000,G=0.011765,B=0.000000,A=1.000000)"))))

(event Custom|DestroyArmour
  (bind _self self)
  (bind _armourpieces (Variables|Default|GetArmourPieces))
  (bind _armourthresholdsindex (Variables|Default|GetArmourThresholdsIndex))
  (bind _armourthresholds (Variables|Default|GetArmourThresholds))
  (bind _armourthresholdsindex_2 (Variables|Default|GetArmourThresholdsIndex))
  (bind _returnvalue (Utilities|GetDisplayName _self))
  (bind _output (Utilities|Array|Get(acopy) _armourpieces _armourthresholdsindex_2))
  ;[1 0 0] Damage the Tank
  (Components|DestroyComponent _output)
  (Utilities|Array|RemoveIndex (Variables|Default|GetArmourPieces) _armourthresholdsindex)
  (Utilities|Array|RemoveIndex _armourthresholds _armourthresholdsindex)
  (if (== (Utilities|Array|Length _armourthresholds) 0)
    (Variables|Default|SetArmour 0.0)
    (bind _output_get (Variables|Default|SetArmourRemaining (Utilities|String|ToString(Float) (Variables|Default|GetArmour))))
    (Development|PrintString (Utilities|String|Append _returnvalue ".ARMOUR: " _output_get) true true "(R=0.219608,G=0.164706,B=0.168627,A=1.000000)")
    (elif (> (stale Custom|DamageArmour _output_get) (Utilities|Array|Get(acopy) (Variables|Default|GetArmourThresholds) (Variables|Default|GetArmourThresholdsIndex)))
      (bind _output_get_2 (Variables|Default|SetArmourRemaining (Utilities|String|ToString(Float) (Variables|Default|GetArmour))))
      (Development|PrintString (Utilities|String|Append _returnvalue ".ARMOUR: " _output_get_2) true true "(R=0.219608,G=0.164706,B=0.168627,A=1.000000)")
      (else
        (Physics|SetSimulatePhysics _output true)
        (Transformation|DetachFromComponent _output "KeepWorld" "KeepWorld" "KeepWorld" true)
        (Utilities|Time|SetTimerbyEvent (delegate Custom|DestroyArmour) 0.05)))))

(event Custom|DamageArmour
  (params (DamageAmount :type Float%20%28double-precision%29))
  (bind _armourpieces (Variables|Default|GetArmourPieces))
  (bind _armourthresholdsindex (Variables|Default|GetArmourThresholdsIndex))
  (bind _output (Utilities|Array|Get(acopy) _armourpieces _armourthresholdsindex))
  ;[1 0 0] Damage the Tank
  (if (< (- (Variables|Default|GetArmour) DamageAmount) 0.0)
    (Variables|Default|SetLeftoverDamage (+ (- (Variables|Default|GetArmour) DamageAmount) (* (- (Variables|Default|GetArmour) DamageAmount) -2.0))))
  (bind _output_get (Variables|Default|SetArmour (- (Variables|Default|GetArmour) DamageAmount)))
  (if (> _output_get (Utilities|Array|Get(acopy) (Variables|Default|GetArmourThresholds) (Variables|Default|GetArmourThresholdsIndex)))
    (bind _output_get_2 (Variables|Default|SetArmourRemaining (Utilities|String|ToString(Float) (Variables|Default|GetArmour))))
    (Development|PrintString (Utilities|String|Append (Utilities|GetDisplayName self) ".ARMOUR: " _output_get_2) true true "(R=0.219608,G=0.164706,B=0.168627,A=1.000000)")
    (else
      (Physics|SetSimulatePhysics _output true)
      (Transformation|DetachFromComponent _output "KeepWorld" "KeepWorld" "KeepWorld" true)
      (Utilities|Time|SetTimerbyEvent (delegate Custom|DestroyArmour) 0.05))))

(event EventBeginPlay
  ;[1 1 1] Begin Play
  (Variables|Default|SetSpawnLocation (Transformation|GetActorLocation))
  (bind _returnvalue (Game|SpawnActorfromClass "/Game/CatBoomerShooter/Weapons/Guns/BP_GrenadeLauncher.BP_GrenadeLauncher_C" (Transformation|GetActorTransform) "AlwaysSpawn" "MultiplyWithRoot" self 0))
  (Variables|Default|SetWeapon _returnvalue)
  (Variables|Default|SetArmourPieces (Utilities|Array|MakeArray (Variables|Default|GetArmourArmRight) (Variables|Default|GetArmourArmLeft) (Variables|Default|GetArmourLegRight) (Variables|Default|GetArmourLegLeft) (Variables|Default|GetArmourHelmet) (Variables|Default|GetArmourChest))))

(event Game|Damage|EventAnyDamage
  (params (Damage :type Float%20%28single-precision%29) (DamageType :type Damage%20Type%20Object%20Reference) (InstigatedBy :type Controller%20Object%20Reference) (DamageCauser :type Actor%20Object%20Reference))
  ;[1 0 0] Damage the Tank
  (Class|AISenseDamage|ReportDamageEvent self InstigatedBy Damage (Transformation|GetActorLocation (Game|GetPlayerCharacter 0)) "0, 0, 0" "None")
  (if (== (Variables|Default|GetArmour) 0.0)
    (CallFunction|DamageHealth Damage (Variables|Default|GetLeftoverDamage))
    (else
      (CallFunction|DamageArmour Damage))))

(fn ConstructionScript)

(fn GetDamageType
  (params (DamageTypes :type E_DamageTypes%20Enum :default "NewEnumerator0"))
  (bind _output_get (Variables|Default|SetDamage (Utilities|Select :Index DamageTypes :NewEnumerator0 1e+01 :NewEnumerator1 4e+01 :NewEnumerator2 17.0 :NewEnumerator3 85.0)))
  (return _output_get))

(fn GetPatrolRoute
  (return (Variables|Default|GetPatrolRoute)))

(fn SetMovementSpeed
  (params (MovementSpeeds :type E_MovementSpeeds%20Enum :default "NewEnumerator0"))
  (bind _output_get (Variables|/Script/Engine.CharacterMovementComponent|SetMaxWalkSpeed (Variables|Character|GetCharacterMovement) (Utilities|Select :Index MovementSpeeds :NewEnumerator0 125.0 :NewEnumerator1 375.0)))
  (return _output_get))