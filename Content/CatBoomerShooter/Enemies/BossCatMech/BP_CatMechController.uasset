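; AI controller for the cat mech boss that runs its behavior tree and detects when the player camps in one spot.
; StartBoss launches the tree, stores the player pawn in the blackboard and starts a looping position-check timer.
; Each check adds a strike if the player stays near the last recorded position, resetting once they move far enough.
; Reaching the strike limit sets the PlayerCamping blackboard flag and resets the count.
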(event Custom|CheckPlayerPos
  (if (> (Math|Vector|Distance(Vector) (Transformation|GetActorLocation (Game|Player|GetPlayerPawn 0)) (Variables|PlayerTracking|GetLastPlayerPos)) (Variables|Default|GetPlayerCampingDistance))
    (Variables|PlayerTracking|SetStrikes 0)
    (Variables|PlayerTracking|SetLastPlayerPos (Transformation|GetActorLocation (Game|Player|GetPlayerPawn 0)))
    (else
      (bind _result (Math|Integer|IncrementInt (Variables|PlayerTracking|GetStrikes))
        (:%20%20
          (Development|PrintString "Strike")
          (if (>= _result (Variables|PlayerTracking|GetMaxStrikes))
            (CallFunction|PlayerCamping)
            (Variables|PlayerTracking|SetStrikes 0)))))))

(event Custom|PlayerCamping
  (AI|Components|Blackboard|SetValueasBool (AI|GetBlackboard 0) (Utilities|Name|MakeLiteralName "PlayerCamping") true))

(event Custom|StartBoss
  (Development|PrintString "Starting the boss")
  (AI|RunBehaviorTree "/Game/CatBoomerShooter/Enemies/BossCatMech/BT_CatMechBoss.BT_CatMechBoss")
  (AI|Components|Blackboard|SetValueasObject (AI|GetBlackboard 0) (Utilities|Name|MakeLiteralName "Player") (Game|Player|GetPlayerPawn 0))
  (Utilities|Time|SetTimerbyEvent (delegate Custom|CheckPlayerPos) (Variables|PlayerTracking|GetCheckPlayerTimer) true))

(event EventBeginPlay)

(fn ConstructionScript)