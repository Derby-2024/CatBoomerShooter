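; BP_HomingMissile is a homing projectile for the BossCatMech enemy's custom attacks.
; Tick steers it toward ActorTarget with interpolated look-at rotation until TrackTime runs out, while moving it forward without sweep.
; It destroys itself and draws a debug sphere on expiry or overlap with a BasePlayerCharacter, applying no damage.
; ActorTarget is not assigned by any live logic here.
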(event OnComponentBeginOverlap(Capsule)
  (params (OverlappedComponent :type Primitive%20Component%20Object%20Reference) (OtherActor :type Actor%20Object%20Reference) (OtherComp :type Primitive%20Component%20Object%20Reference) (OtherBodyIndex :type Integer) (bFromSweep :type Boolean) (SweepResult :type Hit%20Result%20Structure%20%28by%20ref%29))
  (Utilities|Casting|CastToBasePlayerCharacter OtherActor)
  (Actor|DestroyActor)
  (Rendering|Debug|DrawDebugSphere (Transformation|GetActorLocation) 1e+02 12 "(R=0.890757,G=0.024775,B=1.000000,A=1.000000)" 2.0 1e+01))

(event Custom|MissileExpire
  (Actor|DestroyActor)
  (Rendering|Debug|DrawDebugSphere (Transformation|GetActorLocation) 1e+02 12 "(R=0.890757,G=0.024775,B=1.000000,A=1.000000)" 2.0 1e+01))

(event EventTick
  (params (DeltaSeconds :type Float%20%28single-precision%29))
  (Utilities|FlowControl|Sequence
    (:then_0
      (if (Variables|Default|GetTrackActor)
        (Utilities|FlowControl|Sequence
          (:then_0
            (bind _output_get (Variables|Default|SetTrackTime (- (Variables|Default|GetTrackTime) DeltaSeconds)))
            (if (<= _output_get 0.0)
              (Variables|Default|SetTrackActor false)))
          (:then_1
            ;[1 1 1] Comment
            (Transformation|SetActorRotation (Math|Interpolation|RInterpTo (Transformation|GetActorRotation) (Math|Rotator|FindLookatRotation (Transformation|GetActorLocation) (Transformation|GetActorLocation (Variables|Default|GetActorTarget))) DeltaSeconds (Variables|Default|GetTurnSpeed)))))))
    (:then_1
      ;[1 1 1] Comment
      (Transformation|SetActorLocation (+ (Transformation|GetActorLocation) (* (Transformation|GetActorForwardVector) (Variables|Default|GetMoveSpeed) DeltaSeconds)) false false))))

(event EventBeginPlay
  (Utilities|Time|SetTimerbyEvent (delegate Custom|MissileExpire) (Variables|Default|GetExpireTimer)))

(fn ConstructionScript)