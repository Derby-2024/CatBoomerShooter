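; BP_Mortar is a delayed area-of-effect strike actor for the CatMech boss's custom attacks.
; On BeginPlay it sizes its RadialForce, starts a warning timer and traces downward to draw a debug cylinder telegraphing the blast radius on the surface below.
; Fire applies falloff radial damage at the actor's location, ignoring its owner, adds a radial impulse, then destroys the actor.
; Both telegraph and explosion visuals use debug draws.
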(event Custom|Fire
  (bind _returnvalue (Transformation|GetActorLocation))
  (bind _returnvalue_2 (Components|GetOwner))
  (bind _radius (Variables|Default|GetRadius))
  (Rendering|Debug|DrawDebugSphere _returnvalue 2e+02 12 "(R=1.000000,G=0.476097,B=0.000000,A=1.000000)" 0.5 1e+01)
  (Class|GameplayStatics|ApplyRadialDamagewithFalloff (Variables|Default|GetDamage) (Variables|Default|GetMinimumDamage) _returnvalue (* _radius 0.2) _radius 1.0 0 (Utilities|Array|MakeArray _returnvalue_2) self (AI|GetAIController _returnvalue_2) "ECC_Visibility")
  (Class|RadialForceComponent|FireImpulse (Variables|Default|GetRadialForce))
  (Actor|DestroyActor))

(event EventBeginPlay
  (bind _returnvalue (Transformation|GetActorLocation))
  (Variables|/Script/Engine.RadialForceComponent|SetRadius (Variables|Default|GetRadialForce) (Variables|Default|GetRadius))
  (Utilities|FlowControl|DelayUntilNextTick)
  (Utilities|Time|SetTimerbyEvent (EventDispatchers|CreateEvent :!event Custom|Fire) (Variables|Default|GetWarningTime))
  (bind _outhit (Collision|LineTraceByChannel _returnvalue (+ _returnvalue (* (Transformation|GetActorUpVector) -1e+03)) "TraceTypeQuery1" false 0 "None"))
  (Class|KismetSystemLibrary|DrawDebugCylinder (.Location (Collision|BreakHitResult _outhit)) (Math|Vector|MakeVector (.X (Math|Vector|BreakVector (.Location (Collision|BreakHitResult _outhit)))) (.Y (Math|Vector|BreakVector (.Location (Collision|BreakHitResult _outhit)))) (+ (.Z (Math|Vector|BreakVector (.Location (Collision|BreakHitResult _outhit)))) 3e+01)) (Variables|Default|GetRadius) 12 "(R=1.000000,G=0.000000,B=0.195551,A=1.000000)" (Variables|Default|GetWarningTime) 2e+01))

(fn ConstructionScript)