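; BP_MechLaser is a continuous laser attack for the cat mech boss.
; Each tick it traces forward against WorldStatic and Pawn objects, ignoring its parent actor, and damages the hit actor by LaserDPS scaled by delta time.
; The owner's AI controller is passed as damage instigator.
; The beam is shown only with debug drawing, as a red line ending at the impact point or maximum range.
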(fn ConstructionScript)

(fn ReceiveTick
  (params (DeltaSeconds :type Float%20%28single-precision%29))
  (bind _returnvalue (Transformation|GetActorForwardVector))
  (bind _returnvalue_2 (Transformation|GetActorLocation))
  (bind _returnvalue_3 (* _returnvalue 9999.0))
  (bind _returnvalue_4 (+ _returnvalue_2 _returnvalue_3))
  (bind (_outhit _returnvalue_5) (Collision|LineTraceForObjects _returnvalue_2 _returnvalue_4 (Utilities|Array|MakeArray "ObjectTypeQuery1" "ObjectTypeQuery3") false (Utilities|Array|MakeArray (Actor|GetParentActor)) "ForOneFrame"))
  (Rendering|Debug|DrawDebugLine _returnvalue_2 (select _returnvalue_5 (.ImpactPoint (Collision|BreakHitResult _outhit)) _returnvalue_4) "(R=1.000000,G=0.000000,B=0.000000,A=1.000000)" 0.0 1e+01)
  (if _returnvalue_5
    (Game|Damage|ApplyDamage (.HitActor (Collision|BreakHitResult _outhit)) (* (Variables|Default|GetLaserDPS) DeltaSeconds) (AI|GetAIController (Components|GetOwner (Variables|Default|GetScene))) self)))