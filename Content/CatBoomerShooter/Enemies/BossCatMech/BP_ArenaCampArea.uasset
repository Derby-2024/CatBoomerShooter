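; An arena trigger volume for the CatMech boss that detects when the player camps inside it.
; Overlap starts or resumes a camp timer, which calls PlayerCamping on every BP_CatMechController when it expires.
; Leaving pauses that timer and starts a return timer, so re-entering before it expires keeps the accumulated camp time, while staying out clears it.
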(event Custom|PlayerCamping
  (Utilities|Time|ClearandInvalidateTimerbyHandle (Variables|Default|GetCampTimerHandle))
  (bind _outactors (Actor|GetAllActorsOfClass "/Game/CatBoomerShooter/Enemies/BossCatMech/BP_CatMechController.BP_CatMechController_C"))
  (for _array_element _outactors
    (Default|PlayerCamping _array_element)))

(event Custom|PlayerLeft
  (Utilities|Time|ClearandInvalidateTimerbyHandle (Variables|Default|GetCampTimerHandle))
  (Utilities|Time|ClearandInvalidateTimerbyHandle (Variables|Default|GetReturnTimerHandle)))

(event Collision|EventActorBeginOverlap
  (params (OtherActor :type Actor%20Object%20Reference))
  (Utilities|Casting|CastToBasePlayerCharacter OtherActor)
  (if (Utilities|Time|IsValidTimerHandle (Variables|Default|GetCampTimerHandle))
    (Utilities|Time|UnpauseTimerbyHandle (Variables|Default|GetCampTimerHandle))
    (Utilities|Time|ClearandInvalidateTimerbyHandle (Variables|Default|GetReturnTimerHandle))
    (else
      (bind _returnvalue (Utilities|Time|SetTimerbyEvent (delegate Custom|PlayerCamping) (Variables|Default|GetCampTimer)))
      (Variables|Default|SetCampTimerHandle _returnvalue))))

(event Collision|EventActorEndOverlap
  (params (OtherActor :type Actor%20Object%20Reference))
  (Utilities|Casting|CastToBasePlayerCharacter OtherActor)
  (Utilities|Time|PauseTimerbyHandle (Variables|Default|GetCampTimerHandle))
  (bind _returnvalue (Utilities|Time|SetTimerbyEvent (delegate Custom|PlayerLeft) (Variables|Default|GetReturnTimer)))
  (Variables|Default|SetReturnTimerHandle _returnvalue))

(fn ConstructionScript)