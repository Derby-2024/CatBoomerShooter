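; BP_CatMechCharacter is the Cat Mech boss character, handling its laser attack, phase changes and defeat reward.
; SetLaserEnabled toggles tick on the Laser child actor and runs a timer that switches it off after 15 seconds, clearing that timer when disabled.
; NextPhaseTrigger passes the boss phase to CallNextPhase.
; On Destroyed, it calls BossDefeated and spawns the mech boss key pickup at its transform.
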(event Custom|SetLaserEnabled
  (params (bEnabled :type Boolean))
  (Actor|Tick|SetActorTickEnabled (Variables|/Script/Engine.ChildActorComponent|GetChildActor (Variables|Default|GetLaser)) bEnabled)
  (if bEnabled
    (bind _returnvalue (Utilities|Time|SetTimerbyEvent (delegate Custom|LaserExpired) 15.0))
    (Variables|Default|SetLaserExpireTimer _returnvalue)
    (else
      (Utilities|Time|ClearandInvalidateTimerbyHandle (Variables|Default|GetLaserExpireTimer)))))

(event Custom|LaserExpired
  (CallFunction|SetLaserEnabled false))

(event Custom|NextPhaseTrigger
  (params (BossPhase :type E_BossPhase%20Enum :default "NewEnumerator0"))
  (Default|CallNextPhase BossPhase))

(event EventDestroyed
  (Default|CallBossDefeated)
  (Game|SpawnActorfromClass "/Game/CatBoomerShooter/Items/BP_KeyPickup_MechBoss.BP_KeyPickup_MechBoss_C" (Transformation|GetActorTransform) "Undefined" "MultiplyWithRoot" 0 0))

(fn ConstructionScript)