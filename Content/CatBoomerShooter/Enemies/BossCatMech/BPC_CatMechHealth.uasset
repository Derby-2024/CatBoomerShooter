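; Health component for the Cat Mech boss that turns death into a phase change.
; On kill it tells BP_CatMechController to start the next phase, or destroys the owner if that controller is absent.
; RefilHealth runs a looping timer that restores health in steps, then clamps it at max, stops and broadcasts HealthRefilled.
; The BeginPlay and damage handlers are empty, and the damage binding is never run.
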(event Custom|OnTakeAnyDamage_Event
  (params (Damage :type Float%20%28single-precision%29) (CurrentHealth :type Float%20%28single-precision%29) (InstigatedBy :type Controller%20Object%20Reference) (DamageCauser :type Actor%20Object%20Reference)))

(event Custom|RefilHealth
  (bind _returnvalue (Utilities|Time|SetTimerbyEvent (delegate Custom|RefillingHealthTick) 0.2 true)))

(event Custom|RefillingHealthTick
  (bind _output_get (Variables|Default|SetHealth (+ (Variables|Default|GetHealth) (/ (Variables|Default|GetMaxHealth) 25.0) 0.0)))
  (if (> _output_get (Variables|Default|GetMaxHealth))
    (Variables|Default|SetHealth (Variables|Default|GetMaxHealth))
    (Utilities|Time|ClearandInvalidateTimerbyHandle (stale Custom|RefilHealth _returnvalue))
    (Default|CallHealthRefilled)))

(event EventBeginPlay)

(event EventOnKill
  (params (FinalInstigator :type Controller%20Object%20Reference) (FinalDamageCauser :type Actor%20Object%20Reference))
  (bind _asbp_cat_mech_controller (Utilities|Casting|CastToBP_CatMechController (AI|GetAIController (Components|GetOwner)))
    (:then
      (Default|StartNextPhase _asbp_cat_mech_controller))
    (:CastFailed
      (Actor|DestroyActor (Components|GetOwner)))))