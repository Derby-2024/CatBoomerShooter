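; BP_TestActor is a damageable test target in the TankGrenadier enemy folder.
; Its RadialDamage event subtracts the received damage from Health and prints the actor's display name with the remaining health.
; When damage would push Health below zero, it clamps Health to zero, prints it and destroys the actor; reaching exactly zero does not destroy it.
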(event Game|Damage|EventRadialDamage
  (params (DamageReceived :type Float%20%28single-precision%29) (DamageType :type Damage%20Type%20Object%20Reference) (Origin :type Vector :default "0, 0, 0") (HitInfo :type Hit%20Result%20Structure%20%28by%20ref%29) (InstigatedBy :type Controller%20Object%20Reference) (DamageCauser :type Actor%20Object%20Reference))
  (bind _self self)
  (bind _returnvalue (Utilities|GetDisplayName _self))
  ;[1 0 0] Damage the Test Actor
  (if (< (- (Variables|Default|GetHealth) DamageReceived) 0.0)
    (bind _output_get (Variables|Default|SetHealth 0.0))
    (bind _output_get_2 (Variables|Default|SetHealthRemaining (Utilities|String|ToString(Float) _output_get)))
    (Development|PrintString (Utilities|String|Append _returnvalue ".HEALTH: " _output_get_2) true true "(R=0.133333,G=1.000000,B=0.000000,A=1.000000)")
    (Actor|DestroyActor)
    (else
      (bind _output_get_3 (Variables|Default|SetHealth (- (Variables|Default|GetHealth) DamageReceived)))
      (bind _output_get_4 (Variables|Default|SetHealthRemaining (Utilities|String|ToString(Float) _output_get_3)))
      (Development|PrintString (Utilities|String|Append _returnvalue ".HEALTH: " _output_get_4) true true "(R=0.133333,G=1.000000,B=0.000000,A=1.000000)"))))

(fn ConstructionScript)