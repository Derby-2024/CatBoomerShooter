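; AI controller for the turret enemy that turns sight and damage perception updates into Blackboard values.
; HandleSight stores the seen actor in SpottedActor and toggles EnemyLost, also writing the stimulus location as a vector to that same SpottedActor key.
; DamageTaken treats the sensed actor as a Controller and records its pawn and location as damage dealer keys.
; Both handlers print debug strings, and no behavior tree is started in these graphs.
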(event OnTargetPerceptionUpdated(AIPerception)
  (params (Actor :type Actor%20Object%20Reference) (Stimulus :type AI%20Stimulus%20Structure))
  ;[1 1 1] Perception
  (bind _returnvalue (Class|AIPerceptionSystem|GetSenseClassforStimulus Stimulus))
  (if (== _returnvalue "/Script/AIModule.AISense_Sight")
    (CallFunction|HandleSight Stimulus Actor)
    (elif (== _returnvalue "/Script/AIModule.AISense_Damage")
      (CallFunction|DamageTaken Stimulus Actor))))

(event EventBeginPlay)

(event EventTick
  (params (DeltaSeconds :type Float%20%28single-precision%29)))

(fn ConstructionScript)

(fn HandleSight
  (params (SightStimulus :type AI%20Stimulus%20Structure) (SensedActor :type Actor%20Object%20Reference))
  (bind (_age _expirationage _strength _stimuluslocation _receiverlocation _tag _bsuccessfullysensed) (Utilities|Struct|BreakAIStimulus SightStimulus))
  (bind _returnvalue (AI|GetBlackboard 0))
  (bind _enemylost (Variables|Default|GetEnemyLost))
  (bind _returnvalue_2 (Class|AIPerceptionSystem|GetSenseClassforStimulus SightStimulus))
  (if (== _returnvalue_2 "/Script/AIModule.AISense_Sight")
    (if _bsuccessfullysensed
      (Development|PrintString "Enemy sighted!")
      (AI|Components|Blackboard|SetValueasObject (AI|GetBlackboard 0) (Variables|Default|GetSpottedActor) SensedActor)
      (AI|Components|Blackboard|SetValueasBool _returnvalue _enemylost false)
      (AI|Components|Blackboard|SetValueasVector (AI|GetBlackboard 0) (Variables|Default|GetSpottedActor) _stimuluslocation)
      (else
        (Development|PrintString "Lost sight")
        (AI|Components|Blackboard|SetValueasBool _returnvalue _enemylost true)))
    (else
      (return))))

(fn DamageTaken
  (params (DamageStimulus :type AI%20Stimulus%20Structure) (SensedActor :type Actor%20Object%20Reference))
  (bind _ascontroller (Utilities|Casting|CastToController SensedActor))
  (bind _returnvalue (Pawn|GetControlledPawn _ascontroller))
  (bind _returnvalue_2 (Transformation|GetActorLocation _returnvalue))
  (bind _returnvalue_3 (Class|AIPerceptionSystem|GetSenseClassforStimulus DamageStimulus))
  (if (== _returnvalue_3 "/Script/AIModule.AISense_Damage")
    (Development|PrintString "Ouch")
    (AI|Components|Blackboard|SetValueasVector (AI|GetBlackboard 0) (Variables|Default|GetDamageDealerLocation) _returnvalue_2)
    (Development|PrintString (Utilities|String|ToString(Vector) _returnvalue_2))
    (AI|Components|Blackboard|SetValueasObject (AI|GetBlackboard 0) (Variables|Default|GetDamageDealer) _returnvalue)
    (else
      (return))))