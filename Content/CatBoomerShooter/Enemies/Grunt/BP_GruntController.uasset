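; BP_GruntController is the AI controller for the Grunt enemy, turning perception updates into blackboard state.
; Each perception update is routed by sense class to a sight or hearing handler.
; A successful sight or hearing stimulus sets the sensed actor as ActorTarget.
; Losing sight clears the target, flags IsSearching and stores LastKnownLocation; a failed hearing stimulus is ignored, and IsSearching is never reset here.
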(event OnTargetPerceptionUpdated(AIPerception)
  (params (Actor :type Actor%20Object%20Reference) (Stimulus :type AI%20Stimulus%20Structure))
  (bind _returnvalue (Class|AIPerceptionSystem|GetSenseClassforStimulus Stimulus))
  (if (== _returnvalue "/Script/AIModule.AISense_Sight")
    (CallFunction|HandleSight Actor Stimulus)
    (elif (== _returnvalue "/Script/AIModule.AISense_Hearing")
      (CallFunction|HandleHearing Actor Stimulus))))

(event EventBeginPlay)

(event EventTick
  (params (DeltaSeconds :type Float%20%28single-precision%29)))

(fn ConstructionScript)

(fn HandleSight
  (params (Actor :type Actor%20Object%20Reference) (Stimulus :type AI%20Stimulus%20Structure))
  (if (.bSuccessfullySensed (Utilities|Struct|BreakAIStimulus Stimulus))
    (Development|PrintText "Player has been spotted")
    (AI|Components|Blackboard|SetValueasObject (AI|GetBlackboard 0) (Utilities|Name|MakeLiteralName "ActorTarget") Actor)
    (else
      (Development|PrintString "Searching")
      (AI|Components|Blackboard|SetValueasObject (AI|GetBlackboard 0) (Utilities|Name|MakeLiteralName "ActorTarget") 0)
      (AI|Components|Blackboard|SetValueasBool (AI|GetBlackboard 0) (Utilities|Name|MakeLiteralName "IsSearching") true)
      (Development|PrintString "Searching set")
      (AI|Components|Blackboard|SetValueasVector (AI|GetBlackboard 0) (Utilities|Name|MakeLiteralName "LastKnownLocation") (.StimulusLocation (Utilities|Struct|BreakAIStimulus Stimulus))))))

(fn HandleHearing
  (params (Actor :type Actor%20Object%20Reference) (Stimulus :type AI%20Stimulus%20Structure))
  (if (.bSuccessfullySensed (Utilities|Struct|BreakAIStimulus Stimulus))
    (Development|PrintText "Player has been spotted")
    (AI|Components|Blackboard|SetValueasObject (AI|GetBlackboard 0) (Utilities|Name|MakeLiteralName "ActorTarget") (Variables|Default|GetActor))
    (else
      (return))))