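; AI controller for the Bomber enemy that runs the BT_bomber behavior tree on begin play and feeds it perception results.
; Perception updates branch on sense class and write to the blackboard.
; Gaining sight stores the spotted actor; losing it clears the actor, flags searching and saves the last known location.
; Sensed damage stores the stimulus location as the damage location.
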(event OnTargetPerceptionUpdated(AIPerception)
  (params (Actor :type Actor%20Object%20Reference) (Stimulus :type AI%20Stimulus%20Structure))
  (bind (_age _expirationage _strength _stimuluslocation _receiverlocation _tag _bsuccessfullysensed) (Utilities|Struct|BreakAIStimulus Stimulus))
  (bind _returnvalue (AI|GetBlackboard 0))
  (bind _returnvalue_2 (Utilities|Name|MakeLiteralName "Spottedactor"))
  (bind _returnvalue_3 (Class|AIPerceptionSystem|GetSenseClassforStimulus Stimulus))
  (Utilities|FlowControl|Sequence
    (:then_0
      ;[1 1 1] Sight
      (if (== _returnvalue_3 "/Script/AIModule.AISense_Sight")
        (if _bsuccessfullysensed
          (AI|Components|Blackboard|SetValueasObject _returnvalue _returnvalue_2 Actor)
          (else
            (AI|Components|Blackboard|SetValueasObject _returnvalue _returnvalue_2 0)
            (AI|Components|Blackboard|SetValueasBool _returnvalue (Utilities|Name|MakeLiteralName "Searching") true)
            (AI|Components|Blackboard|SetValueasVector _returnvalue (Utilities|Name|MakeLiteralName "Lastknownlocation") _stimuluslocation)))))
    (:then_1
      ;[1 1 1] Damage
      (if (== _returnvalue_3 "/Script/AIModule.AISense_Damage")
        (if _bsuccessfullysensed
          (AI|Components|Blackboard|SetValueasVector (AI|GetBlackboard 0) (Utilities|Name|MakeLiteralName "Damage location") _stimuluslocation))))))

(event EventBeginPlay
  (AI|RunBehaviorTree "/Game/CatBoomerShooter/Enemies/Bomber/BT_bomber.BT_bomber"))

(fn ConstructionScript)