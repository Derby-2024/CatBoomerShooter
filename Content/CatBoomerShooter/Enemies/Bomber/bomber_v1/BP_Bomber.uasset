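; BP_Bomber is a bomber enemy character whose bomb explodes with particles, sound, a radial impulse and radial damage, then destroys the actor.
; Bomb overlap detonates immediately; deathboom removes the mesh, launches the physics-simulated bomb along current velocity and detonates after a delay.
; Enableunstable makes any actor hit trigger detonation.
; An Elite flag swaps material, speed and blast stats at BeginPlay, though damage radius stays hardcoded, ignoring BombRadius.
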(event OnComponentBeginOverlap(Bomb)
  (params (OverlappedComponent :type Primitive%20Component%20Object%20Reference) (OtherActor :type Actor%20Object%20Reference) (OtherComp :type Primitive%20Component%20Object%20Reference) (OtherBodyIndex :type Integer) (bFromSweep :type Boolean) (SweepResult :type Hit%20Result%20Structure%20%28by%20ref%29))
  ;[1 1 1] Bomb hit
  (Variables|Default|SetDelay 0.0)
  (CallFunction|Boom))

(event Custom|Boom
  ;[1 1 1] Bomb detination
  (Utilities|FlowControl|Delay (Variables|Default|GetDelay))
  (CallFunction|Boominstant))

(event Custom|BecomeElite
  (bind _explosive_force (Variables|Default|GetExplosive%20force))
  ;[1 1 1] Elite
  (Rendering|Material|SetMaterial (Variables|Character|GetMesh) 2 "/Game/CatBoomerShooter/Enemies/Bomber/bomber_v1/M_Elitebody.M_Elitebody")
  (bind _output_get (Variables|/Script/Engine.CharacterMovementComponent|SetMaxWalkSpeed (Variables|Character|GetCharacterMovement) (Variables|Default|GetElite%20Walk%20Speed)))
  (Variables|Default|SetDefault%20speed _output_get)
  (Variables|/Script/Engine.RadialForceComponent|SetRadius _explosive_force (Variables|Default|GetElite%20Radius))
  (Variables|/Script/Engine.RadialForceComponent|SetImpulseStrength _explosive_force (Variables|Default|GetElite%20Impulse%20Strength))
  (Variables|Default|SetBomb%20damage (Variables|Default|GetElite%20Bomb%20Damage))
  (Variables|Default|SetBomb%20radius (Variables|Default|GetElite%20Bomb%20Radius)))

(event Custom|Unstablecollide
  (params (SelfActor :type Actor%20Object%20Reference) (OtherActor :type Actor%20Object%20Reference) (NormalImpulse :type Vector) (Hit :type Hit%20Result%20Structure%20%28by%20ref%29))
  ;[1 1 1] Collide
  (CallFunction|Boominstant))

(event Custom|Enableunstable
  ;[1 1 1] Collide
  (Collision|BindEventtoOnActorHit (delegate Custom|Unstablecollide)))

(event Custom|deathboom
  (bind _returnvalue (Transformation|GetVelocity))
  (bind (_x _y _z) (Class|KismetMathLibrary|BreakVector3f _returnvalue))
  ;[1 1 1] death
  (Physics|SetSimulatePhysics (Variables|Default|GetBomb) true)
  (Components|DestroyComponent (Variables|Character|GetMesh))
  (Variables|Default|SetDelay 3.0)
  (Physics|AddImpulse (Variables|Default|GetBomb) (Math|Vector|MakeVector (/ _x 5.0) (/ _y 5.0) (/ _z 5.0)) "None" false)
  (CallFunction|Boom))

(event Custom|Boominstant
  (bind _bomb (Variables|Default|GetBomb))
  (bind _returnvalue (Transformation|GetWorldLocation _bomb))
  ;[1 1 1] Bomb detination
  (Effects|SpawnEmitteratLocation "/Engine/Tutorial/SubEditors/TutorialAssets/TutorialParticleSystem.TutorialParticleSystem" _returnvalue)
  (Audio|PlaySoundatLocation "/Engine/VREditor/Sounds/VR_ungrab.VR_ungrab" _returnvalue "0, 0, 0" 1.0 1.0 0.0 0 0 0 0)
  (Class|RadialForceComponent|FireImpulse (Variables|Default|GetExplosive%20force))
  (Game|Damage|ApplyRadialDamage (Variables|Default|GetBomb%20damage) _returnvalue 3e+02 0 0 0 0 false "ECC_Visibility")
  (Actor|DestroyActor))

(event EventBeginPlay
  ;[1 1 1] Start
  (if (Variables|Default|GetElite?)
    (CallFunction|BecomeElite)))

(fn ConstructionScript)

(fn Updatespeed
  (params (New%20speed :type Float%20%28double-precision%29))
  (Variables|/Script/Engine.CharacterMovementComponent|SetMaxWalkSpeed (Variables|Character|GetCharacterMovement) New%20speed))

(fn NewFunction
  (params (A :type Vector)))