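; AI controller for the bomber enemy that starts the BT_bomber behavior tree on BeginPlay.
; AI Perception updates drive the Spottedactor blackboard key, setting it when an actor tagged Player is sensed by sight.
; The key is cleared when sight of the player is lost or when any non-sight stimulus arrives.
; Both outcomes print a debug message.
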(event OnTargetPerceptionUpdated(AIPerception)
  (params (Actor :type Actor%20Object%20Reference) (Stimulus :type AI%20Stimulus%20Structure))
  (bind _returnvalue (AI|GetBlackboard 0))
  (bind _returnvalue_2 (Utilities|Name|MakeLiteralName "Spottedactor"))
  (bind _returnvalue_3 (Class|AIPerceptionSystem|GetSenseClassforStimulus Stimulus))
  (if (== _returnvalue_3 "/Script/AIModule.AISense_Sight")
    (if (Actor|ActorHasTag Actor "Player")
      (if (.bSuccessfullySensed (Utilities|Struct|BreakAIStimulus Stimulus))
        (AI|Components|Blackboard|SetValueasObject _returnvalue _returnvalue_2 Actor)
        (Development|PrintString "spotted")
        (else
          (AI|Components|Blackboard|SetValueasObject _returnvalue _returnvalue_2 0 :!label _label)
          (Development|PrintString "lost"))))
    (else
      (goto _label))))

(event EventBeginPlay
  (AI|RunBehaviorTree "/Game/CatBoomerShooter/AI_Bomber/BT_bomber.BT_bomber"))

(fn ConstructionScript)