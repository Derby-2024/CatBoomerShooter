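; Grenade projectile for the CatBoomerShooter guns that explodes whenever the actor is destroyed.
; On BeginPlay its sphere collider ignores the owning actor while moving.
; The Destroyed event spawns a separate particle actor, fires a radial force impulse at the grenade's location and applies radial damage with falloff, ignoring itself.
; Debug sphere draws for visualizing the radius are present but disconnected.
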(event EventBeginPlay
  ;[0.2969 0.2969 0.2969] Ignore Owner Actor
  (Collision|IgnoreActorwhenMoving (Variables|Default|GetSphereCollider) (Components|GetOwner) true))

(event EventDestroyed
  (bind _returnvalue (Transformation|GetActorLocation))
  (bind _radialforce (Variables|Default|GetRadialForce))
  ;[0 0.9849 1] Spawn Particle System When Destroyed
  (Game|SpawnActorfromClass "/Game/CatBoomerShooter/Enemies/TankGrenade/BP_GrenadeParticles.BP_GrenadeParticles_C" (Transformation|GetActorTransform) "Undefined" "MultiplyWithRoot" 0 0)
  (Transformation|SetWorldLocation _radialforce _returnvalue false false)
  (Class|RadialForceComponent|FireImpulse _radialforce)
  (Class|GameplayStatics|ApplyRadialDamagewithFalloff 25.0 1e+01 _returnvalue 1e+02 4e+02 1.0 "/Script/Engine.DamageType" (Utilities|Array|MakeArray self) 0 0 "ECC_Visibility"))

(fn ConstructionScript)