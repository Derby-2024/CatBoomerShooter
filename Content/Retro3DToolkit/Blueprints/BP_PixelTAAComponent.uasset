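; Pixel TAA component that switches anti-aliasing and sharpening according to player camera movement, in the Retro 3D Toolkit.
; Each tick it compares camera location and forward vector with the previous frame against movement and rotation thresholds.
; While moving, it either raises AA quality or lowers the TAA current-frame weight, depending on ToggleAA, and removes sharpening.
; When still, AA turns off or frame weight and sharpening return to maximum, all via per-tick console commands.
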(event EventTick
  (params (DeltaSeconds :type Float%20%28single-precision%29))
  (bind _playerindex (Variables|Default|GetPlayerIndex))
  (bind _returnvalue (Game|GetPlayerCameraManager _playerindex))
  (bind _returnvalue_2 (Camera|GetCameraLocation _returnvalue))
  (bind _returnvalue_3 (Camera|GetCameraRotation _returnvalue))
  ;[1 1 1] Change Anti-Aliasing Settings when the Camera Moves
  (Utilities|FlowControl|Sequence
    (:then_0
      (if (Variables|Default|GetbToggleAA)
        (|SetToggleAA (or (> (Math|Vector|VectorLengthSquared (- (Variables|Default|GetCameraLocation) _returnvalue_2)) (Variables|Default|GetMinCameraMoveDist)) (> (* (Math|Vector|VectorLength (- (Math|Rotator|GetRotationXVector (Variables|Default|GetCameraRotation)) (Math|Rotator|GetRotationXVector _returnvalue_3))) 1e+03) (Variables|Default|GetMinCameraRotationDist))))
        (else
          (|SetTemporalAA (or (> (Math|Vector|VectorLengthSquared (- (Variables|Default|GetCameraLocation) _returnvalue_2)) (Variables|Default|GetMinCameraMoveDist)) (> (* (Math|Vector|VectorLength (- (Math|Rotator|GetRotationXVector (Variables|Default|GetCameraRotation)) (Math|Rotator|GetRotationXVector _returnvalue_3))) 1e+03) (Variables|Default|GetMinCameraRotationDist)))))))
    (:then_1
      (|ImageSharpen (or (> (Math|Vector|VectorLengthSquared (- (Variables|Default|GetCameraLocation) _returnvalue_2)) (Variables|Default|GetMinCameraMoveDist)) (> (* (Math|Vector|VectorLength (- (Math|Rotator|GetRotationXVector (Variables|Default|GetCameraRotation)) (Math|Rotator|GetRotationXVector _returnvalue_3))) 1e+03) (Variables|Default|GetMinCameraRotationDist)))))
    (:then_2
      (Variables|Default|SetCameraLocation _returnvalue_2)
      (Variables|Default|SetCameraRotation _returnvalue_3))))